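; FlyHat is a flying target actor that shuttles back and forth and awards score to players who damage it.
; Each tick, Movement sweeps it along the normalized Direction at Speed, reversing Direction whenever its countdown timer expires.
; Any damage casts the instigator's PlayerState to MyPlayerState and calls IncrementScore2, even on the failed-cast branch.
; The construction script sets the root component to replicate.
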(event EventTick
  (params (DeltaSeconds :type Float%20%28single-precision%29))
  (CallFunction|Movement))

(event Game|Damage|EventAnyDamage
  (params (Damage :type Float%20%28single-precision%29) (DamageType :type Damage%20Type%20Object%20Reference) (InstigatedBy :type Controller%20Object%20Reference) (DamageCauser :type Actor%20Object%20Reference))
  (bind _asmy_player_state (Utilities|Casting|CastToMyPlayerState (Variables|/Script/Engine.Controller|GetPlayerState InstigatedBy))
    (:then
      _)
    (:CastFailed
      _))
  (Default|IncrementScore2 _asmy_player_state))

(fn ConstructionScript
  (Class|ActorComponent|SetIsReplicated (Variables|Default|GetDefaultSceneRoot) true))

(fn Movement
  (bind _output_get (Variables|Default|SetOBJPosition (Transformation|GetActorLocation)))
  (Transformation|SetActorLocation (+ _output_get (* (Math|Vector|Normalize (Variables|Default|GetDirection)) (* (Utilities|Time|GetWorldDeltaSeconds) (Variables|Default|GetSpeed)))) true true)
  (Variables|Default|SetTime (- (Variables|Default|GetTime) (Utilities|Time|GetWorldDeltaSeconds)))
  (if (>= 0.0 (Variables|Default|GetTime))
    (Variables|Default|SetDirection (Math|Vector|NegateVector (Variables|Default|GetDirection)))
    (Variables|Default|SetTime 5.0)))